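; BP_NPC_AI is the AI controller for guard NPCs, driving their behavior through perception and a behavior tree.
; On BeginPlay it sets up the PatrolData blackboard, runs the GuardBehaviour tree and caches the blackboard component.
; Perception updates for actors without the "Enemy" tag write the sensed actor to EnemyKey, or clear that key when sensing fails.
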(event `self.ReceiveBeginPlay`
  (bind _blackboardcomponent (`self.UseBlackboard` "/Game/Dynamic/NPC/AI/PatrolData.PatrolData"))
  (`self.RunBehaviorTree` "/Game/Dynamic/NPC/AI/GuardBehaviour.GuardBehaviour")
  (set `self.BlackBoardComp.` _blackboardcomponent))

(event `self.AIPerception.OnTargetPerceptionUpdated`
  (params (Actor :type "Actor Object Reference") (Stimulus :type "AIStimulus Structure"))
  (bind _blackboardcomp_ (`self.BlackBoardComp.`))
  (bind _enemykey (`self.EnemyKey`))
  (if (`self.ActorHasTag` Actor "Enemy")
    _
    (elif (`.bSuccessfullySensed` (break `AIStimulus` Stimulus))
      (`BlackboardComponent.SetValueAsObject` _blackboardcomp_ _enemykey Actor)
      (else
        (`BlackboardComponent.ClearValue` _blackboardcomp_ _enemykey)))))

(fn `UserConstructionScript`)